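; Player-controlled physics ball that is aimed and launched with the mouse, with camera look, slow motion and a points widget.
; LaunchVelocity scales the deprojected cursor direction by VectorMultiplier, forcing Z upward.
; Pressing StartShoot draws a one-frame predicted path, using that velocity offset by the sphere's world location; releasing adds the velocity to the sphere.
; Holding slowTime lowers global time dilation until release.
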(event Custom|Aiming
  (bind _sphere (Variables|Default|GetSphere))
  (bind _returnvalue (Transformation|GetWorldLocation _sphere))
  ;[1 1 1] Shoot and Predict
  (Class|GameplayStatics|BlueprintPredictProjectilePathbyTraceChannel _returnvalue (+ _returnvalue (CallFunction|LaunchVelocity)) true 5.0 "ECC_WorldStatic" true 0 "ForOneFrame" 1e+01 15.0 2.0 2.0))

(event EventBeginPlay
  ;[1 1 1] Score Widget
  (bind _returnvalue (UserInterface|CreateWidget "/Game/Blueprints/WBP_Points.WBP_Points_C"))
  (UserInterface|Viewport|AddtoViewport _returnvalue 0))

(event Input|ActionEvents|InputActionStartShoot
  (params (Key :type Key%20Structure :default "None"))
  ;[1 1 1] Shoot and Predict
  (:Pressed
    (CallFunction|Aiming))
  (:Released
    (Physics|SetPhysicsLinearVelocity (Variables|Default|GetSphere) (CallFunction|LaunchVelocity) true "None")))

(event Input|ActionEvents|InputActionslowTime
  (params (Key :type Key%20Structure :default "None"))
  ;[1 1 1] Time Slow
  (:Pressed
    (Utilities|Time|SetGlobalTimeDilation 0.1))
  (:Released
    (Utilities|Time|SetGlobalTimeDilation 1.0)))

(event Input|AxisEvents|InputAxisTurnLeft/Right
  (params (AxisValue :type Float%20%28single-precision%29))
  ;[1 1 1] Camera Movement
  (Pawn|Input|AddControllerYawInput AxisValue))

(event Input|AxisEvents|InputAxisLookUp,Up
  (params (AxisValue :type Float%20%28single-precision%29))
  ;[1 1 1] Camera Movement
  (Pawn|Input|AddControllerPitchInput AxisValue))

(fn ConstructionScript)

(fn LaunchVelocity
  (bind _returnvalue (Game|GetPlayerController 0))
  (bind _vectormultiplier (Variables|Default|GetVectorMultiplier))
  (bind _worlddirection (Game|Player|ConvertMouseLocationToWorldSpace _returnvalue))
  (bind _returnvalue_2 (Math|Vector|Normalize _worlddirection))
  (bind _returnvalue_3 (* (.z _returnvalue_2) _vectormultiplier))
  (return (Math|Vector|MakeVector (* (.x _returnvalue_2) _vectormultiplier) (* (.y _returnvalue_2) _vectormultiplier) (Math|Float|SelectFloat _returnvalue_3 (* _returnvalue_3 -1.0) (> (.z _returnvalue_2) 0.0)))))