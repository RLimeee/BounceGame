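; BP_splinePathway is an actor that moves a cube along its spline path, starting at BeginPlay.
; A timeline's float track lerps distance from zero to the spline's length, setting the cube's world location without sweep each update.
; When the timeline finishes, it waits briefly and calls Play without explicitly rewinding.
; Tick prints the world location of a single spline point, apparently for debugging.
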(event EventBeginPlay
  (bind _newtrack_0 (Timeline|Timeline_0 PlayFromStart)
    (:Update
      (bind _output_get (Variables|Default|Setlocation (Spline|GetLocationatDistanceAlongSpline (Variables|Default|GetSpline) (Math|Float|Lerp 0.0 (Spline|GetSplineLength (Variables|Default|GetSpline)) _newtrack_0) "World")))
      (Transformation|SetWorldLocation (Variables|Default|GetCube) _output_get false false))
    (:Finished
      (Utilities|FlowControl|Delay 3.0)
      (Timeline|Timeline_0 Play))))

(event Collision|EventActorBeginOverlap
  (params (OtherActor :type Actor%20Object%20Reference)))

(event EventTick
  (params (DeltaSeconds :type Float%20%28single-precision%29))
  (Development|PrintString (Utilities|String|ToString(Vector) (Spline|GetLocationatSplinePoint (Variables|Default|GetSpline) 1 "World"))))

(fn ConstructionScript)