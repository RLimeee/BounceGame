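; Ball actor component that clips walls between the player camera and its owner.
; A looping timer drives a multi object trace along the camera's forward vector, as long as the camera-to-owner distance.
; Hit actors are tracked in current and previous wall arrays, toggling the "ClipSize" material parameter on their static mesh.
; When the trace finds nothing, a DoOnce unclips the current walls and empties both arrays.
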(event Custom|CheckOverlap
  (bind (_start_trace _end_trace) (CallFunction|ComputeTrace))
  (bind (_outhits _returnvalue) (Class|KismetSystemLibrary|LineTraceMultiforObjects _start_trace _end_trace (Utilities|Array|MakeArray "ObjectTypeQuery7") false 0 "None" true))
  (if _returnvalue
    (for _array_element _outhits
      (bind _output_get (Variables|Default|SetCurrent%20Wall (.HitActor (Collision|BreakHitResult _array_element))))
      (if (not (Utilities|Array|ContainsItem (Variables|Default|GetcurrentWalls) _output_get))
        (Utilities|Array|AddUnique (Variables|Default|GetcurrentWalls) (Variables|Default|GetCurrent%20Wall))
        (for _array_element_2 (Variables|Default|GetcurrentWalls)
          (CallFunction|WallClip _array_element_2 true))
        (for _array_element_3 (Variables|Default|GetpreviousWalls)
          (CallFunction|WallClip _array_element_3 false))
        (else
          (Variables|Default|SetpreviousWalls (Variables|Default|GetcurrentWalls)))))
    (CallFunction|ResetLineTrace)
    (else
      (Utilities|FlowControl|DoOnce false
        (:Completed
          (for _array_element_4 (Variables|Default|GetcurrentWalls)
            (CallFunction|WallClip _array_element_4 false))
          (Utilities|Array|Clear (Variables|Default|GetpreviousWalls))
          (Utilities|Array|Clear (Variables|Default|GetcurrentWalls)))))))

(event Custom|Reset%20Line%20Trace
  (Utilities|FlowControl|DoOnce false) ; enters at Reset
)

(event EventBeginPlay
  (Utilities|Time|SetTimerbyEvent (EventDispatchers|CreateEvent :!event Custom|CheckOverlap) 0.2 true))

(fn ComputeTrace
  (bind _returnvalue (Game|GetPlayerCameraManager 0))
  (bind _returnvalue_2 (Game|GetPlayerCameraManager 0))
  (bind _returnvalue_3 (Camera|GetCameraLocation _returnvalue))
  (return _returnvalue_3 (+ _returnvalue_3 (* (Math|Vector|GetForwardVector (Camera|GetCameraRotation _returnvalue_2)) (Math|Vector|Distance(Vector) (Camera|GetCameraLocation _returnvalue_2) (Transformation|GetActorLocation (Components|GetOwner)))))))

(fn WallClip
  (params (Wall :type Actor%20Object%20Reference) (Clip :type Boolean))
  (Utilities|IsValid (Actor|GetComponentbyClass Wall "/Script/Engine.StaticMeshComponent")
    (:Is%20Valid
      (Rendering|Material|SetScalarParameterValueonMaterials (Actor|GetComponentbyClass Wall "/Script/Engine.StaticMeshComponent") "ClipSize" (Math|Conversions|ToFloat(Boolean) Clip))
      (return))))