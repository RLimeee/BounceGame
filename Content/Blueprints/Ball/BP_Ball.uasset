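; Player-controlled physics ball that rolls by acceleration forces on its Sphere from movement axes and adds a WBP_Line widget at BeginPlay.
; Look axes drive controller rotation, with Up/Down mapped to yaw and Left/Right to pitch.
; A slow-motion pull-and-release shot with path prediction, using mouse-deprojected LaunchVelocity, exists but is disconnected.
; Interact is empty, and Left/Right movement prints a debug string.
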(event EventBeginPlay
  ;[1 1 1] Shoot and Predict
  (bind _returnvalue (UserInterface|CreateWidget "/Game/Blueprints/UI/WBP_Line.WBP_Line_C"))
  (UserInterface|Viewport|AddtoViewport _returnvalue 0))

(event Input|ActionEvents|InputActionStartShoot
  (params (Key :type Key%20Structure))
  ;[1 1 1] Shoot and Predict
)

(event Input|AxisEvents|InputAxisForward/Backwards
  (params (AxisValue :type Float%20%28single-precision%29))
  (Physics|AddForce (Variables|Default|GetSphere) (Math|Vector|MakeVector 0.0 (* AxisValue 1e+01) 0.0) "None" true))

(event Input|AxisEvents|InputAxisLeft/Right
  (params (AxisValue :type Float%20%28single-precision%29))
  (Physics|AddForce (Variables|Default|GetSphere) (Math|Vector|MakeVector (* AxisValue 1e+01) 0.0 0.0) "None" true)
  (Development|PrintString "Hello"))

(event Input|AxisEvents|InputAxisLookLeft/Right
  (params (AxisValue :type Float%20%28single-precision%29))
  ;[1 1 1] Camera Movement
  (Pawn|Input|AddControllerPitchInput AxisValue))

(event Input|AxisEvents|InputAxisLookUp/Down
  (params (AxisValue :type Float%20%28single-precision%29))
  ;[1 1 1] Camera Movement
  (Pawn|Input|AddControllerYawInput AxisValue))

(fn ConstructionScript)

(fn LaunchVelocity
  (bind _returnvalue (Game|GetPlayerController 0))
  (bind _vectormultiplier (Variables|Default|GetVectorMultiplier))
  (bind _worlddirection (Game|Player|ConvertMouseLocationToWorldSpace _returnvalue))
  (bind _returnvalue_2 (Math|Vector|Normalize _worlddirection))
  (bind _returnvalue_3 (* (.z _returnvalue_2) _vectormultiplier))
  (return (Math|Vector|MakeVector (* (.x _returnvalue_2) _vectormultiplier) (* (.y _returnvalue_2) _vectormultiplier) (Math|Float|SelectFloat _returnvalue_3 (* _returnvalue_3 -1.0) (> (.z _returnvalue_2) 0.0)))))

(fn Interact)