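; BP_BouncyWall is a one-shot bumper that scores and launches a BP_Ball entering its Box trigger.
; The first ball overlap calls Score on the BounceMode game mode and plays a timeline that moves the Cube along Z.
; Each timeline update pushes the ball along the Arrow and turns the red Cube black.
; The first end overlap reverses the timeline; neither DoOnce gate is reset.
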(event OnComponentBeginOverlap(Box)
  (params (OverlappedComponent :type Primitive%20Component%20Object%20Reference) (OtherActor :type Actor%20Object%20Reference) (OtherComp :type Primitive%20Component%20Object%20Reference) (OtherBodyIndex :type Integer) (bFromSweep :type Boolean) (SweepResult :type Hit%20Result%20Structure%20%28by%20ref%29))
  (bind _asbp_ball (Utilities|Casting|CastToBP_Ball OtherActor))
  (Utilities|FlowControl|DoOnce false
    (:Completed
      (Utilities|FlowControl|Sequence
        (:then_0
          (bind _asbounce_mode (Utilities|Casting|CastToBounceMode (Game|GetGameMode)))
          (Default|Score _asbounce_mode))
        (:then_1
          (bind _moveboard (Timeline|Timeline_0 Play)
            (:Update
              (Transformation|SetRelativeLocation (Variables|Default|GetCube) (Math|Vector|MakeVector 0.0 0.0 (* _moveboard 1e+01)) false false)
              (Physics|AddImpulse (Variables|/Game/Blueprints/BP_Ball.BP_Ball_C|GetSphere _asbp_ball) (* (Math|Vector|GetForwardVector (Variables|Default|GetArrow)) 1e+03) "None" true)
              (Rendering|Material|SetVectorParameterValueonMaterials (Variables|Default|GetCube) "Color" "0, 0, 0"))))))))

(event OnComponentEndOverlap(Box)
  (params (OverlappedComponent :type Primitive%20Component%20Object%20Reference) (OtherActor :type Actor%20Object%20Reference) (OtherComp :type Primitive%20Component%20Object%20Reference) (OtherBodyIndex :type Integer))
  (Utilities|FlowControl|DoOnce false
    (:Completed
      (bind _moveboard (Timeline|Timeline_0 Reverse)
        (:Update
          (Transformation|SetRelativeLocation (Variables|Default|GetCube) (Math|Vector|MakeVector 0.0 0.0 (* _moveboard 1e+01)) false false)
          (Physics|AddImpulse (Variables|/Game/Blueprints/BP_Ball.BP_Ball_C|GetSphere (stale OnComponentBeginOverlap(Box) _asbp_ball)) (* (Math|Vector|GetForwardVector (Variables|Default|GetArrow)) 1e+03) "None" true)
          (Rendering|Material|SetVectorParameterValueonMaterials (Variables|Default|GetCube) "Color" "0, 0, 0"))))))

(fn ConstructionScript
  (Rendering|Material|SetVectorParameterValueonMaterials (Variables|Default|GetCube) "Color" "1.000000, 0, 0"))