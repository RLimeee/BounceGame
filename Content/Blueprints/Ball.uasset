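; Ball Blueprint that computes a launch velocity from where the mouse cursor points.
; LaunchVelocity deprojects player 0's cursor into a world direction, normalizes it and scales it by VectorMultipler.
; The Z sign is flipped when not positive, so a positive multiplier always gives a non-downward launch.
; The event graph holds no logic, so nothing here applies the velocity, and Sphere and IsAiming are unused.
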(fn ConstructionScript)

(fn LaunchVelocity
  (bind _returnvalue (Game|GetPlayerController 0))
  (bind _vectormultipler (Variables|Default|GetVectorMultipler))
  (bind _worlddirection (Game|Player|ConvertMouseLocationToWorldSpace _returnvalue))
  (bind _returnvalue_2 (Math|Vector|Normalize _worlddirection))
  (return (Math|Vector|MakeVector (* (.x _returnvalue_2) _vectormultipler) (* (.y _returnvalue_2) _vectormultipler) (Math|Float|SelectFloat (* (.z _returnvalue_2) _vectormultipler) (* (* _vectormultipler -1.0) (.z _returnvalue_2)) (> (.z _returnvalue_2) 0.0)))))