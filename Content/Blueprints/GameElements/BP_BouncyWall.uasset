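; BP_BouncyWall is an interactable wall that scores through the BounceMode game mode and launches an overlapping object.
; Box overlap caches the component; Interact adds score and plays the BacknForth timeline.
; A never-reset DoOnce on the timeline update offsets the Cube once, impulses the cached component along the Arrow, and turns the red Cube black.
; Later interactions can still score but do not launch again.
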(event OnComponentBeginOverlap(Box)
  (params (OverlappedComponent :type Primitive%20Component%20Object%20Reference) (OtherActor :type Actor%20Object%20Reference) (OtherComp :type Primitive%20Component%20Object%20Reference) (OtherBodyIndex :type Integer) (bFromSweep :type Boolean) (SweepResult :type Hit%20Result%20Structure%20%28by%20ref%29))
  (Variables|Default|SetOther%20Comp_0 OtherComp))

(event EventInteract
  (Utilities|FlowControl|Sequence
    (:then_0
      (bind _asbounce_mode (Utilities|Casting|CastToBounceMode (Game|GetGameMode)))
      (Default|Score _asbounce_mode))
    (:then_1
      (bind _moveboard (Timeline|backnForth Play)
        (:Update
          (Utilities|FlowControl|DoOnce false
            (:Completed
              (Transformation|SetRelativeLocation (Variables|Default|GetCube) (Math|Vector|MakeVector 0.0 0.0 (* _moveboard 1e+01)) false false)
              (Physics|AddImpulse (Variables|Default|GetOther%20Comp_0) (* (Math|Vector|GetForwardVector (Variables|Default|GetArrow)) 1e+03) "None" false)
              (Rendering|Material|SetVectorParameterValueonMaterials (Variables|Default|GetCube) "Color" "0, 0, 0")
              (Development|PrintString "fire"))))))))

(fn ConstructionScript
  (Rendering|Material|SetVectorParameterValueonMaterials (Variables|Default|GetCube) "Color" "1.000000, 0, 0"))